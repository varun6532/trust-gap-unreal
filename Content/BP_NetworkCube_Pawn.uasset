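; Networked cube pawn that appears to demonstrate movement cheating and its detection, adding a W_Cheat widget on BeginPlay.
; Pressing W sends the location string over UDP and requests a server move, which nudges the cube forward.
; Server_Mover echoes a requested position over UDP and, past an X threshold, flags Cheating yet still applies it.
; Other server events set location from a parsed string or reset to the saved home; both OnRep functions are empty.
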(event `Server_SendLocation`
  (params (`LocationString ` :type String))
  (bind _returnvalue (`KismetStringLibrary.ParseIntoArray` `LocationString ` ","))
  (`KismetSystemLibrary.PrintString` `LocationString `)
  (`self.K2_SetActorLocation` (`KismetMathLibrary.MakeVector` (`KismetStringLibrary.Conv_StringToDouble` (`|GetArrayItem` _returnvalue)) (`KismetStringLibrary.Conv_StringToDouble` (`|GetArrayItem` _returnvalue 1)) (`KismetStringLibrary.Conv_StringToDouble` (`|GetArrayItem` _returnvalue 2)))))

(event `self.ReceiveBeginPlay`
  (set `self.HomeLocation` (`self.K2_GetActorLocation`))
  (bind _returnvalue (`|CreateWidget` "/Game/W_Cheat.W_Cheat_C"))
  (`UserWidget.AddToViewport` _returnvalue 0))

(event `Key|W`
  (params (Key :type "Key Structure"))
  (bind _returnvalue (`KismetStringLibrary.BuildString_Vector` "" "" (`self.K2_GetActorLocation`)))
  (:`Pressed`
    (`NetworkHelper.SendUDPMessage` _returnvalue)
    (`self.Server_MoveForward` _returnvalue)))

(event `Server_MoveForward`
  (params (`LocationString ` :type String))
  (set `self.Cheating?` false)
  (`KismetSystemLibrary.PrintString` `LocationString `)
  (`self.K2_SetActorLocation` (+ (* (`self.GetActorForwardVector`) (10.0 10.0 10.0)) (`self.K2_GetActorLocation`))))

(event `Server_Mover`
  (params (Location_To_MMove :type "Vector Structure"))
  (`KismetSystemLibrary.PrintString` (`KismetStringLibrary.Conv_VectorToString` Location_To_MMove))
  (`NetworkHelper.SendUDPMessage` (`KismetStringLibrary.Conv_VectorToString` Location_To_MMove))
  (if (> (.x Location_To_MMove) 25.0)
    (set `self.Cheating?` true)
    (`KismetSystemLibrary.PrintString` "YOU ARE CHEATING ")
    (`self.K2_SetActorLocation` Location_To_MMove)
    (set `self.Cheating?` true)))

(event `Server_Reset`
  (set `self.Cheating?` false)
  (`KismetSystemLibrary.PrintString` "Position Reset ")
  (`self.K2_SetActorLocation` (`self.HomeLocation`)))

(fn `OnRep_Cheating?`)

(fn `OnRep_HomeLocation`)

(fn `UserConstructionScript`)